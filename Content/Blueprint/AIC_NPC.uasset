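; AI controller for an NPC that runs BT_Character and feeds it destinations from the pawn's target points or a perceived target.
; GetNextDestination cycles target points by wrapping index, and SetNextDestination writes the location to the blackboard.
; Sensing an actor whose first tag matches TargetName sets a detected flag and starts a fast looping timer copying its location.
; Losing it clears the flag and writes the next point, but never clears the timer.
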(event `self.ReceiveBeginPlay`
  (bind _asbp_ai_character (cast `/Game/Blueprint/BP_AI_Character` (`self.K2_GetPawn`)))
  (set `self.As BP AI Character` _asbp_ai_character)
  (`self.RunBehaviorTree` "/Game/Blueprint/BT_Character.BT_Character")
  (bind _destination (`self.GetNextDestination`))
  (`self.SetNextDestination` _destination))

(event `self.AIPerception.OnTargetPerceptionUpdated`
  (params (Actor :type "Actor Object Reference") (Stimulus :type "AIStimulus Structure"))
  (bind _blackboard (`self.Blackboard`))
  (if (== (`|GetArrayItem` (`Actor.Tags` Actor)) (`self.Target Name`))
    (if (`.bSuccessfullySensed` (break `AIStimulus` Stimulus))
      (`KismetSystemLibrary.PrintString` "Detected")
      (`BlackboardComponent.SetValueAsBool` _blackboard "IsDetected?" true)
      (`KismetSystemLibrary.K2_SetTimerDelegate` (delegate `Set Target Location`) 0.04 true)
      (else
        (`KismetSystemLibrary.PrintString` "Forgot" true true (struct :`R` 1.0 :`B` 0.01037 :`A` 1.0))
        (`BlackboardComponent.SetValueAsBool` _blackboard "IsDetected?" false)
        (bind _destination (`self.GetNextDestination`))
        (`self.SetNextDestination` _destination)))))

(event `Set Target Location`
  (`self.SetNextDestination` (`self.K2_GetActorLocation` (stale `self.AIPerception.OnTargetPerceptionUpdated` Actor))))

(fn `GetNextDestination`
  (returns (Destination :type "Vector Structure"))
  (bind _targets_point (`/Game/Blueprint/BP_AI_Character.Targets_Point` (`self.As BP AI Character`)))
  (bind _output_get (set `self.Current_Target_Point_Index` (+ (`self.Current_Target_Point_Index`) 1)))
  (return (`self.K2_GetActorLocation` (`|GetArrayItem` _targets_point (mod _output_get (`KismetArrayLibrary.Array_Length` _targets_point))))))

(fn `SetNextDestination`
  (params (NewDestination :type "Vector Structure"))
  (`BlackboardComponent.SetValueAsVector` (`self.Blackboard`) (`self.Key Name`) NewDestination))

(fn `UserConstructionScript`)